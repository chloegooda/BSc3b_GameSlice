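; Right-hand transition gate that moves the player between streamed levels while a timeline swings its pivot about yaw.
; Toggle starts the gate animation and a scene transition that pauses player movement, then teleports the player to TeleportLocation after a delay.
; EntranceToLevel selects loading or unloading the enum-named level, then adjusts movement mode through a BP_NPC_QuestGiver cast on the player character.
; An older OpenLevel path remains, unused.
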(event `/Game/ThirdPersonCharacter/BPI_Interact.Toggle`
  (`self.TransitionBetweenScenes`)
  (if (`self.IsOpen`)
    (bind (_direction _timeline) (`Timeline|Timeline_1` :`NewTime` 1.0 :!via `Reverse` :!label _label)
      (:`Update`
        (`SceneComponent.K2_SetRelativeRotation` (`self.Pivot`) (`KismetMathLibrary.MakeRotator` 0.0 0.0 (* _timeline 90.0)) false false))
      (:`Finished`
        (`SceneComponent.K2_SetRelativeRotation` (`self.Pivot`) (`KismetMathLibrary.MakeRotator` 0.0) false false)
        (set `self.IsOpen` false)))
    (else
      (goto _label))))

(event `TransitionBetweenScenes`
  (bind _returnvalue (`GameplayStatics.GetPlayerCharacter` 0))
  (bind _charactermovement (`Character.CharacterMovement` _returnvalue))
  (`ActorComponent.SetActive` _charactermovement false false)
  (`/Game/FX/SceneTransition/FL_PlaySceneTransition.PlaySceneTransition` false)
  (`KismetSystemLibrary.Delay` 1.0)
  (`self.LoadInLevel`)
  (`self.K2_SetActorLocation` _returnvalue (`self.K2_GetActorLocation` (`self.TeleportLocation`)) false false)
  (`ActorComponent.SetActive` _charactermovement true false))

(event `LoadInLevel`
  (bind _returnvalue (`KismetStringLibrary.Conv_StringToName` (`|GetEnumeratorNameAsString` (`self.Level`))))
  (if (`self.EntranceToLevel?`)
    (`GameplayStatics.LoadStreamLevel` _returnvalue true)
    (bind _asbp_npc_quest_giver (cast `/Game/AI/NPCs/BaseClasses/BP_NPC_QuestGiver` (`GameplayStatics.GetPlayerCharacter` 0)))
    (`CharacterMovementComponent.SetMovementMode` (`Character.CharacterMovement` _asbp_npc_quest_giver) "MOVE_Walking" 0)
    (else
      (bind _asbp_npc_quest_giver_2 (cast `/Game/AI/NPCs/BaseClasses/BP_NPC_QuestGiver` (`GameplayStatics.GetPlayerCharacter` 0)))
      (`CharacterMovementComponent.DisableMovement` (`Character.CharacterMovement` _asbp_npc_quest_giver_2))
      (`GameplayStatics.UnloadStreamLevel` _returnvalue))))

(fn `UserConstructionScript`
  (`parent.UserConstructionScript`))