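; BP_PlayerDoor is a door that swings on its pivot and loads another level.
; Toggle plays or reverses a timeline based on IsOpen, driving the pivot's yaw through up to 90 degrees.
; When the timeline finishes, it flips IsOpen and opens the level named by the LevelToOpen enum, converted from string to name.
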(event `/Game/ThirdPersonCharacter/BPI_Interact.Toggle`
  (if (`self.IsOpen`)
    (bind (_direction _timeline) (`Timeline|Timeline_0` :`NewTime` 1.0 :!via `Reverse` :!label _label)
      (:`Update`
        (`SceneComponent.K2_SetRelativeRotation` (`self.Pivot`) (`KismetMathLibrary.MakeRotator` 0.0 0.0 (* _timeline 90.0)) false false))
      (:`Finished`
        (set `self.isOpen` (not (`self.isOpen`)))
        (`GameplayStatics.OpenLevel` (`KismetStringLibrary.Conv_StringToName` (`|GetEnumeratorNameAsString` (`self.LevelToOpen`))))))
    (else
      (goto _label))))

(fn `UserConstructionScript`)