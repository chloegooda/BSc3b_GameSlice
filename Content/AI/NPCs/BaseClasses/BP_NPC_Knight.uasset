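; BP_NPC_Knight is a knight NPC that walks an endless patrol loop through four patrol points, starting on BeginPlay at its configured walk speed.
; Patrol chains AI move requests through fixed array indices, pausing briefly at each stop before calling itself again; no failure path is handled.
; At each stop, Rotate casts the current point to NPC_POI and snaps the knight's yaw toward that point's linked item.
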(event `Patrol`
  (bind _output (`|GetArrayItem` (`self.Patrol Points`) 3))
  (bind _output_2 (`|GetArrayItem` (`self.Patrol Points`)))
  (bind _output_3 (`|GetArrayItem` (`self.Patrol Points`) 1))
  (bind _output_4 (`|GetArrayItem` (`self.Patrol Points`) 2))
  (set `self.Target POI` _output_2)
  (`|AIMoveTo` self (0.0 0.0 0.0) _output_2
    (:`OnSuccess`
      (`self.Rotate`)
      (`KismetSystemLibrary.Delay` 2.0)
      (set `self.Target POI` _output_3)
      (`|AIMoveTo` self (0.0 0.0 0.0) _output_3
        (:`OnSuccess`
          (`self.Rotate`)
          (`KismetSystemLibrary.Delay` 2.0)
          (set `self.Target POI` _output_4)
          (`|AIMoveTo` self (0.0 0.0 0.0) _output_4
            (:`OnSuccess`
              (`self.Rotate`)
              (`KismetSystemLibrary.Delay` 2.0)
              (set `self.Target POI` _output)
              (`|AIMoveTo` self (0.0 0.0 0.0) _output
                (:`OnSuccess`
                  (`self.Rotate`)
                  (`KismetSystemLibrary.Delay` 2.0)
                  (`self.Patrol`))))))))))

(event `self.ReceiveBeginPlay`
  (bind _speed (`self.Speed`))
  (set `CharacterMovementComponent.MaxWalkSpeed` _speed (`self.CharacterMovement`))
  (`KismetSystemLibrary.PrintString` (`KismetStringLibrary.Conv_DoubleToString` _speed))
  (`self.Patrol`))

(event `Rotate`
  (bind _asnpc_poi (cast `/Game/AI/POIS/NPC_POI` (`self.Target POI`)))
  (bind (_returnvalue_roll _returnvalue_pitch _returnvalue_yaw) (`KismetMathLibrary.BreakRotator` (`KismetMathLibrary.FindLookAtRotation` (`self.K2_GetActorLocation`) (`self.K2_GetActorLocation` (`/Game/AI/POIS/NPC_POI.Linked Item` _asnpc_poi)))))
  (`self.K2_SetActorRotation` (`KismetMathLibrary.MakeRotator` 0.0 0.0 _returnvalue_yaw)))

(fn `UserConstructionScript`)