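; BP_NPC_Seller is a seller NPC that opens a shop screen when the player character overlaps its ShopTrigger.
; On overlap it blends the player's view to itself, then after a short delay shows BPW_Seller with UI-only input and a visible cursor.
; It also hides the player character and moves it to a hard-coded world location; restoring view, input and visibility is not handled here.
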(event `self.Shop Trigger.OnComponentBeginOverlap`
  (params (OverlappedComponent :type "PrimitiveComponent Object Reference") (OtherActor :type "Actor Object Reference") (OtherComp :type "PrimitiveComponent Object Reference") (OtherBodyIndex :type Integer) (bFromSweep :type Boolean) (SweepResult :type "HitResult Structure (by ref)"))
  (bind _returnvalue (`GameplayStatics.GetPlayerController` 0))
  (if (== OtherActor (`GameplayStatics.GetPlayerCharacter` 0))
    (`PlayerController.SetViewTargetWithBlend` _returnvalue self 2.0 "VTBlend_Linear" 0.0 false)
    (`KismetSystemLibrary.Delay` 2.2)
    (bind _returnvalue_2 (`|CreateWidget` "/Game/UI/BPW_Seller.BPW_Seller_C"))
    (`UserWidget.AddToViewport` _returnvalue_2 0)
    (`WidgetBlueprintLibrary.SetInputMode_UIOnlyEx` _returnvalue _returnvalue_2)
    (set `PlayerController.bShowMouseCursor` true _returnvalue)
    (`self.SetActorHiddenInGame` (`GameplayStatics.GetPlayerCharacter` 0) true)
    (`self.K2_SetActorLocation` (`GameplayStatics.GetPlayerCharacter` 0) (-140.0 -10.0 86.0) false false)))

(fn `UserConstructionScript`)