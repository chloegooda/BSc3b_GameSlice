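; Villager peasant man NPC Blueprint that sets its name to "Villager" on BeginPlay, then runs the parent's BeginPlay.
; On Interact, it casts player character 0 to PlayerCharacter and calls CallInteracted on every quest in that player's quest log, passing itself.
; The construction script only calls its parent, and the overlap and Tick events are unused.
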(event `/Game/QuestSystem/Blueprints/BPI_QuestInteractInterface.Interact`
  (bind _asplayer_character (cast `/Game/ThirdPersonCharacter/PlayerCharacter` (`GameplayStatics.GetPlayerCharacter` 0)))
  (for _array_element (`/Game/QuestSystem/Blueprints/BP_QuestLog.Quests` (`/Game/ThirdPersonCharacter/PlayerCharacter.BP_QuestLog` _asplayer_character))
    (`/Game/QuestSystem/Quests/BP_Quest.Interacted` _array_element self)))

(event `self.ReceiveBeginPlay`
  (set `self.Name` "Villager")
  (`parent.ReceiveBeginPlay`))

(fn `UserConstructionScript`
  (`parent.UserConstructionScript`))