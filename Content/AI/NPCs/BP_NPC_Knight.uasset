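; BP_NPC_Knight is a knight NPC Blueprint that walks a patrol route when play begins.
; BeginPlay calls the Patrol event, which chains AIMoveTo calls through the first four PatrolPoints actors, pausing briefly after each successful arrival.
; The chain is hardcoded by index and does not loop, so the route runs once and no further move follows a failed one.
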(event `Patrol`
  (`|AIMoveTo` self (0.0 0.0 0.0) (`|GetArrayItem` (`self.Patrol Points`))
    (:`OnSuccess`
      (`KismetSystemLibrary.Delay` 2.0)
      (`|AIMoveTo` self (0.0 0.0 0.0) (`|GetArrayItem` (`self.Patrol Points`) 1)
        (:`OnSuccess`
          (`KismetSystemLibrary.Delay` 2.0)
          (`|AIMoveTo` self (0.0 0.0 0.0) (`|GetArrayItem` (`self.Patrol Points`) 2)
            (:`OnSuccess`
              (`KismetSystemLibrary.Delay` 2.0)
              (`|AIMoveTo` self (0.0 0.0 0.0) (`|GetArrayItem` (`self.Patrol Points`) 3)
                (:`OnSuccess`
                  (`KismetSystemLibrary.Delay` 2.0))))))))))

(event `self.ReceiveBeginPlay`
  (`self.Patrol`))

(fn `UserConstructionScript`)