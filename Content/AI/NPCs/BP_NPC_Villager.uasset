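; Villager NPC that wanders endlessly between random market stall points of interest.
; On BeginPlay it gathers NPC_POI actors tagged "Market Stall", then starts a recursive AIMoveTo loop toward random picks.
; On arrival it yaws toward the POI's LinkedItem, waits a random few seconds, prints another random POI's name and moves again.
; Only a successful move continues the loop, as failure is unhandled.
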(event `Move`
  (bind _random_poi (`self.Get Random POI`))
  (`|AIMoveTo` self (0.0 0.0 0.0) _random_poi
    (:`OnSuccess`
      (`self.Rotate`)
      (`KismetSystemLibrary.Delay` (`KismetMathLibrary.RandomFloatInRange` 3.0 8.0))
      (`KismetSystemLibrary.PrintString` (`KismetSystemLibrary.GetDisplayName` _random_poi) true true (struct :`R` 0.340115 :`B` 1.0 :`A` 1.0))
      (`self.Move`))))

(event `self.ReceiveBeginPlay`
  (`|ExecutionSequence`
    (:`then_0`
      (bind _outactors (`GameplayStatics.GetAllActorsOfClassWithTag` "/Game/AI/POIS/NPC_POI.NPC_POI_C" "Market Stall"))
      (set `self.NPC Points of Interest` _outactors))
    (:`then_1`
      (`self.Move`))))

(event `Rotate`
  (bind _asnpc_poi (cast `/Game/AI/POIS/NPC_POI` (`self.Target POI`)))
  (bind (_returnvalue_roll _returnvalue_pitch _returnvalue_yaw) (`KismetMathLibrary.BreakRotator` (`KismetMathLibrary.FindLookAtRotation` (`self.K2_GetActorLocation`) (`self.K2_GetActorLocation` (`/Game/AI/POIS/NPC_POI.Linked Item` _asnpc_poi)))))
  (`self.K2_SetActorRotation` (`KismetMathLibrary.MakeRotator` 0.0 0.0 _returnvalue_yaw)))

(fn `Get Random POI`
  (returns (`Random POI` :type "TargetPoint Object Reference"))
  (bind _npc_points_of_interest (`self.NPC Points of Interest`))
  (bind _output_get (set `self.Target POI` (`|GetArrayItem` _npc_points_of_interest (`KismetMathLibrary.RandomIntegerInRange` 0 (- (`KismetArrayLibrary.Array_Length` _npc_points_of_interest) 1)))))
  (return _output_get))

(fn `UserConstructionScript`)